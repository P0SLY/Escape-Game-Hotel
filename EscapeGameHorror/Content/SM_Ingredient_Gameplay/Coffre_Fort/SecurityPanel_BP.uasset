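; Security panel Blueprint for a safe (coffre), showing a password screen and opening the safe on a correct code.
; On BeginPlay it binds UseKeypad to the first-person character's MErde event dispatcher.
; UseKeypad creates the password widget with a reference to the panel, then switches to UI-only input with a visible cursor.
; CorrectPassword tells the linked CoffreBP to open; the password check itself lives outside this Blueprint.
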(event `self.ReceiveBeginPlay`
  (bind _asbp_first_person_character (cast `/Game/StoryAdvTemplate/Blueprints/BP_FirstPersonCharacter` (`GameplayStatics.GetPlayerCharacter` 0)))
  (add `/Game/StoryAdvTemplate/Blueprints/BP_FirstPersonCharacter.MErde` _asbp_first_person_character (delegate `Use Keypad`)))

(event `Use Keypad`
  (bind _returnvalue (`GameplayStatics.GetPlayerController` 0))
  (bind _returnvalue_2 (`|CreateWidget` "/Game/UI_Folde/Password_Screen_UI.Password_Screen_UI_C"))
  (set `/Game/UI_Folde/Password_Screen_UI.SecurityPanelBp` self _returnvalue_2)
  (`UserWidget.AddToViewport` _returnvalue_2 0)
  (`WidgetBlueprintLibrary.SetInputMode_UIOnlyEx` _returnvalue _returnvalue_2)
  (set `PlayerController.bShowMouseCursor` true _returnvalue))

(event `Correct Password`
  (`/Game/SM_Ingredient_Gameplay/Coffre_Fort/Coffre_BP.Open COffre` (`self.CoffreBP`)))

(fn `UserConstructionScript`)