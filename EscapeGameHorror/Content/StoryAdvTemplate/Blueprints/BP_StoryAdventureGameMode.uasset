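; Game mode for the story adventure template that shows the HUD and runs a minutes-and-seconds countdown.
; BeginPlay adds UI_HUD, while a one-second Delay on Tick paces the countdown and minute rollover.
; A game-over branch adds the GameOver widget, hides the cursor and pauses.
; That branch is unreachable as written, because it requires zero seconds inside the negative-seconds check.
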(event `self.ReceiveBeginPlay`
  (bind _returnvalue (`|CreateWidget` "/Game/StoryAdvTemplate/UserInterface/UI_HUD.UI_HUD_C"))
  (`UserWidget.AddToViewport` _returnvalue 0))

(event `self.ReceiveTick`
  (params (DeltaSeconds :type "Float (single-precision)"))
  (`KismetSystemLibrary.Delay` 1.0)
  (set `self.TimeSec` (- (`self.TimeSec`) 1))
  (if (< (`self.TimeSec`) 0)
    (set `self.TimeMin` (- (`self.TimeMin`) 1))
    (if (and (== (`self.TimeMin`) 0) (== (`self.TimeSec`) 0))
      (bind _returnvalue (`|CreateWidget` "/Game/StoryAdvTemplate/UserInterface/GameOver.GameOver_C"))
      (`UserWidget.AddToViewport` _returnvalue 0)
      (set `PlayerController.bShowMouseCursor` false (`GameplayStatics.GetPlayerController` 0))
      (`GameplayStatics.SetGamePaused` true)
      (else
        (set `self.TimeSec` 59)))))

(fn `UserConstructionScript`)